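; BP_EnemyPartolBox is a trigger actor that tells a group of patrol enemies when a player enters or leaves its area.
; Overlapping actors count as players if they implement BPI_Player.
; On begin overlap, each valid entry in PatrolActors receives that actor as its combat target.
; On end overlap, the same entries get SetCombatTarget with no target, clearing it even if another player remains inside.
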(event `self.ReceiveActorBeginOverlap`
  (params (OtherActor :type "Actor Object Reference"))
  (if (`KismetSystemLibrary.DoesImplementInterface` OtherActor "/Game/Blueprints/Interfaces/BPI_Player.BPI_Player_C")
    (for _array_element (`self.PatrolActors`)
      (`/Engine/EditorBlueprintResources/StandardMacros.IsValid` _array_element
        (:`Is Valid`
          (`/Game/Blueprints/Interfaces/BPI_Enemy.SetCombatTarget` _array_element OtherActor))))))

(event `self.ReceiveActorEndOverlap`
  (params (OtherActor :type "Actor Object Reference"))
  (if (`KismetSystemLibrary.DoesImplementInterface` OtherActor "/Game/Blueprints/Interfaces/BPI_Player.BPI_Player_C")
    (for _array_element (`self.PatrolActors`)
      (`/Engine/EditorBlueprintResources/StandardMacros.IsValid` _array_element
        (:`Is Valid`
          (`/Game/Blueprints/Interfaces/BPI_Enemy.SetCombatTarget` _array_element null))))))

(fn `UserConstructionScript`)